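; BP_Ghost is a 2D flipbook ghost that animates by movement state and notifies interactive objects it touches.
; UpdateMovementState maps EMovementState to left or right idle and walk flipbooks, running on construction, BeginPlay and every Tick.
; The state is only read here, never set.
; A Sphere overlap calls OnOverlapMessage on any actor implementing BPI_Interactive.
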(event `self.ReceiveBeginPlay`
  (`parent.ReceiveBeginPlay`)
  (`self.UpdateMovementState`))

(event `self.ReceiveTick`
  (params (DeltaSeconds :type "Float (single-precision)"))
  (`parent.ReceiveTick` DeltaSeconds)
  (`self.UpdateMovementState`))

(event `self.Sphere.OnComponentBeginOverlap`
  (params (OverlappedComponent :type "PrimitiveComponent Object Reference") (OtherActor :type "Actor Object Reference") (OtherComp :type "PrimitiveComponent Object Reference") (OtherBodyIndex :type Integer) (bFromSweep :type Boolean) (SweepResult :type "HitResult Structure (by ref)"))
  (if (`KismetSystemLibrary.DoesImplementInterface` OtherActor "/Game/Blueprints/BPI_Interactive.BPI_Interactive_C")
    (bind _output_get (set `self.Other Actor` OtherActor))
    (message `/Game/Blueprints/BPI_Interactive.OnOverlap` _output_get)))

(fn `UpdateMovementState`
  (if (`|EnumEquality` (`self.E_MovementState`) "NewEnumerator0")
    (`PaperFlipbookComponent.SetFlipbook` (`self.Sprite`) (`self.FP_IdleLeft`))
    (elif (`|EnumEquality` (`self.E_MovementState`) "NewEnumerator1")
      (`PaperFlipbookComponent.SetFlipbook` (`self.Sprite`) (`self.FP_IdleRight`))
      (elif (`|EnumEquality` (`self.E_MovementState`) "NewEnumerator2")
        (`PaperFlipbookComponent.SetFlipbook` (`self.Sprite`) (`self.FP_WalkLeft`))
        (elif (`|EnumEquality` (`self.E_MovementState`) "NewEnumerator3")
          (`PaperFlipbookComponent.SetFlipbook` (`self.Sprite`) (`self.FP_WalkRight`)))))))

(fn `UserConstructionScript`
  (`parent.UserConstructionScript`)
  (`self.UpdateMovementState`))
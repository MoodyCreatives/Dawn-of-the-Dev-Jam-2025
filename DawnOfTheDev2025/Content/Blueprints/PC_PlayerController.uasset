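; Player controller that handles movement input for the player's ghost character (BP_Ghost).
; On BeginPlay it adds the Enhanced Input player mapping context, sets game-only input and caches the ghost reference.
; IA_Move applies movement relative to control yaw, negating the Y axis for sideways motion.
; Set Player State then sets the ghost's movement state only on exact full-axis values, checking X before Y.
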(event `self.ReceiveBeginPlay`
  (bind _returnvalue (pcsubsystem `EnhancedInputLocalPlayerSubsystem` self))
  (`/Engine/EditorBlueprintResources/StandardMacros.IsValid` _returnvalue
    (:`Is Valid`
      (`EnhancedInputSubsystemInterface.AddMappingContext` _returnvalue "/Game/Blueprints/Input/IMC_Player.IMC_Player" 0 (struct))
      (`WidgetBlueprintLibrary.SetInputMode_GameOnly` self)
      (bind _asbp_ghost (cast `/Game/Blueprints/BP_Ghost` (`GameplayStatics.GetPlayerCharacter` 0)))
      (set `self.As BP Ghost` _asbp_ghost))))

(event `EnhancedInput|/Game/Blueprints/Input/IA_Move`
  (params (ActionValue :type "Vector2D Structure") (ElapsedSeconds :type "Float (double-precision)") (TriggeredSeconds :type "Float (double-precision)") (InputAction :type "InputAction Object Reference" :default "/Game/Blueprints/Input/IA_Move.IA_Move"))
  (bind (_returnvalue_roll _returnvalue_pitch _returnvalue_yaw) (`KismetMathLibrary.BreakRotator` (`self.GetControlRotation`)))
  (bind (_returnvalue_roll_2 _returnvalue_pitch_2 _returnvalue_yaw_2) (`KismetMathLibrary.BreakRotator` (`self.GetControlRotation`)))
  (bind _returnvalue (`GameplayStatics.GetPlayerPawn` 0))
  (bind _returnvalue_2 (* ActionValue_Y -1.0))
  (:`Triggered`
    (`Pawn.AddMovementInput` _returnvalue (`KismetMathLibrary.GetRightVector` (`KismetMathLibrary.MakeRotator` 0.0 0.0 _returnvalue_yaw)) _returnvalue_2 false)
    (`Pawn.AddMovementInput` _returnvalue (`KismetMathLibrary.GetForwardVector` (`KismetMathLibrary.MakeRotator` 0.0 0.0 _returnvalue_yaw_2)) ActionValue_X false)
    (`self.Set Player State` ActionValue_X _returnvalue_2)))

(fn `Set Player State`
  (params (X :type "Float (double-precision)") (Y :type "Float (double-precision)"))
  (if (== X -1.0)
    (set `/Game/Blueprints/BP_Base_Character.E_MovementState` "NewEnumerator2" (`self.As BP Ghost`))
    (elif (== X 1.0)
      (set `/Game/Blueprints/BP_Base_Character.E_MovementState` "NewEnumerator3" (`self.As BP Ghost`))
      (elif (== Y 1.0)
        (set `/Game/Blueprints/BP_Base_Character.E_MovementState` "NewEnumerator0" (`self.As BP Ghost`))
        (elif (== Y -1.0)
          (set `/Game/Blueprints/BP_Base_Character.E_MovementState` "NewEnumerator3" (`self.As BP Ghost`)))))))

(fn `UserConstructionScript`)
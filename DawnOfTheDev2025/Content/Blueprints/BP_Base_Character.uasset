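; BP_Base_Character is a base character Blueprint that shows a 2D flipbook sprite matching its movement state.
; UpdateMovementState maps the EMovementState value to idle-left, idle-right, walk-left or walk-right flipbooks through chained branches and applies the result to the Sprite.
; Only the Construction Script calls it, and the event graph holds empty events plus an unconnected AddMovementInput, so no runtime movement logic runs here.
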(event `self.ReceiveBeginPlay`)

(event `self.ReceiveTick`
  (params (DeltaSeconds :type "Float (single-precision)")))

(fn `UpdateMovementState`
  (if (`|EnumEquality` (`self.E_MovementState`) "NewEnumerator0")
    (`PaperFlipbookComponent.SetFlipbook` (`self.Sprite`) (`self.FP_IdleLeft`))
    (elif (`|EnumEquality` (`self.E_MovementState`) "NewEnumerator1")
      (`PaperFlipbookComponent.SetFlipbook` (`self.Sprite`) (`self.FP_IdleRight`))
      (elif (`|EnumEquality` (`self.E_MovementState`) "NewEnumerator2")
        (`PaperFlipbookComponent.SetFlipbook` (`self.Sprite`) (`self.FP_WalkLeft`))
        (elif (`|EnumEquality` (`self.E_MovementState`) "NewEnumerator3")
          (`PaperFlipbookComponent.SetFlipbook` (`self.Sprite`) (`self.FP_WalkRight`)))))))

(fn `UserConstructionScript`
  (`self.UpdateMovementState`))